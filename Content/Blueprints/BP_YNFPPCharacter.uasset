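; BP_YNFPPCharacter is a first-person character Blueprint that limits how far the camera can pitch up and down.
; Each Tick, when the character is locally viewed, it checks the player camera manager's pitch against fixed upper and lower limits.
; Past either limit, it sets FPSCameraComponent's world rotation to the clamped pitch, keeping yaw and roll; control rotation is not modified.
; BeginPlay, overlap and the construction script do nothing.
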(event `self.ReceiveTick`
  (params (DeltaSeconds :type "Float (single-precision)"))
  (bind _returnvalue (`self.IsLocallyViewed`))
  (bind _fpscameracomponent (`self.FPSCameraComponent`))
  (bind _roll (.roll (`PlayerCameraManager.GetCameraRotation` (`GameplayStatics.GetPlayerCameraManager` 0))))
  (bind _pitch (.pitch (`PlayerCameraManager.GetCameraRotation` (`GameplayStatics.GetPlayerCameraManager` 0))))
  (bind _yaw (.yaw (`PlayerCameraManager.GetCameraRotation` (`GameplayStatics.GetPlayerCameraManager` 0))))
  ;[0.4546 0.4205 1] 限制相机俯仰角
  (if (and _returnvalue (> _pitch 75.0))
    (`SceneComponent.K2_SetWorldRotation` _fpscameracomponent (`KismetMathLibrary.MakeRotator` _roll 75.0 _yaw) false false)
    (elif (and _returnvalue (< _pitch -60.0))
      (`SceneComponent.K2_SetWorldRotation` _fpscameracomponent (`KismetMathLibrary.MakeRotator` _roll -60.0 _yaw) false false))))

(fn `UserConstructionScript`)